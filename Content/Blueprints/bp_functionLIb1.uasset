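; Blueprint function library of helpers for a square-grid map, covering tile lookup and enum stepping.
; GetGridSquareFromCoords linearly searches a given array for the square with matching coordinates.
; GetSurroundingTiles reads the player controller's flattened GridArray and collects valid tiles in a square block offset by R, its side summed from 1 to R.
; GetNextEnum is meant to return the following enum value with wraparound, but clears its working array before looping over it.
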(fn `getGridSquareFromCoords`
  (params (gridSquareArray :type "Array of /Game/Blueprints/bp_gridSquare Object Reference") (coords :type "Vector Structure"))
  (returns (`Array Element` :type "/Game/Blueprints/bp_gridSquare Object Reference"))
  (for _array_element gridSquareArray
    (if (== (`/Game/Blueprints/bp_gridSquare.currentCoords` _array_element) coords)
      (return _array_element))))

(fn `getNextEnum`
  (params (enum :type Byte))
  (returns (nextEnum :type Byte))
  (locals (tempEnum :type "Array of Byte"))
  (bind _tempenum (`local.tempEnum`))
  (bind _tempenum_2 (`local.tempEnum`))
  (bind _returnvalue (+ (`KismetArrayLibrary.Array_Find` _tempenum enum) 1))
  (`KismetArrayLibrary.Array_Clear` _tempenum)
  (for _array_element _tempenum
    (`KismetArrayLibrary.Array_Add` (`local.tempEnum`) _array_element))
  (if (<= _returnvalue (`KismetArrayLibrary.Array_Length` _tempenum))
    (return (`|GetArrayItem` _tempenum_2 _returnvalue))
    (else
      (return (`|GetArrayItem` _tempenum_2)))))

(fn `getSurroundingTiles`
  (params (R1 :type Integer) (X1 :type Integer) (Y1 :type Integer))
  (returns (surroundingTiles :type "Array of /Game/Blueprints/bp_gridSquare Object Reference"))
  (locals (R :type Integer) (X :type Integer) (Y :type Integer) (I :type Integer :default 2) (tiles :type "Array of /Game/Blueprints/bp_gridSquare Object Reference") (playerControllerRef :type "/Game/Blueprints/controllers/bp_ctlr_player Object Reference"))
  (bind _playercontrollerref (`local.playerControllerRef`))
  (bind _i (`local.I`))
  (set `local.R` R1)
  (set `local.X` (- X1 (`local.R`)))
  (set `local.Y` (- Y1 (`local.R`)))
  (bind _asbp_ctlr_player (cast `/Game/Blueprints/controllers/bp_ctlr_player` (`GameplayStatics.GetPlayerController` null)))
  (set `local.playerControllerRef` _asbp_ctlr_player)
  (for _index (range 1 (+ (`local.R`) 1))
    (set `local.I` (+ (`local.I`) _index)))
  (for _index_2 (range (* _i _i))
    (bind _output (`|GetArrayItem` (`/Game/Blueprints/controllers/bp_ctlr_player.gridArray` _playercontrollerref) (+ (+ (mod _index_2 (`local.I`)) (`local.X`)) (* (+ (/ _index_2 (`local.I`)) (`local.Y`)) (`/Game/Blueprints/controllers/bp_ctlr_player.gridHorizontal` _playercontrollerref)))))
    (`/Engine/EditorBlueprintResources/StandardMacros.IsValid` _output
      (:`Is Valid`
        (`KismetArrayLibrary.Array_Add` (`local.tiles`) _output))))
  (return (`local.tiles`)))